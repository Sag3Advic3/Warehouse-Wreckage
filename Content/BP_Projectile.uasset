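; BP_Projectile is a projectile actor that is fired by physics rather than a movement component.
; Launch applies a velocity-change impulse to the static mesh along the actor's forward vector and plays an explosion sound at its location.
; A separate PrintYourName function prints the actor's display name, and the event graph holds only disabled stub events.
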(event EventBeginPlay)

(event Collision|EventActorBeginOverlap
  (params (OtherActor :type Actor%20Object%20Reference)))

(event EventTick
  (params (DeltaSeconds :type Float%20%28single-precision%29)))

(fn ConstructionScript)

(fn PrintYourName
  (Development|PrintString (Utilities|GetDisplayName self)))

(fn Launch
  (bind _self self)
  (Physics|AddImpulse (Variables|/Script/Engine.StaticMeshActor|GetStaticMeshComponent _self) (* (Transformation|GetActorForwardVector _self) 2e+03) "None" true)
  (Audio|PlaySoundatLocation "/Game/StarterContent/Audio/Explosion02.Explosion02" (Transformation|GetActorLocation) "0, 0, 0" 1.0 1.0 0.0 0 0 0 0))